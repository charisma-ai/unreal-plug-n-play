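; Manager actor that shows on-screen speech textboxes for female Charisma NPCs.
; On BeginPlay it creates a hidden W_Textbox per NPC, keyed by the NPC's TextBoxTransform, and passes both lists to a CharismaTextboxHelper C++ component.
; Each tick it sets name and message, shows boxes while their Duration counts down, and flags whether each projected anchor is within the viewport.
; The helper then updates widget screen positions.
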(event `self.ReceiveBeginPlay`
  (bind _textboxmap (`self.TextboxMap`))
  (`|ExecutionSequence`
    (:`then_0`
      ;[1 1 1] Finds all TextBox transforms and instantiates a UMG Textbox Widget
      (bind _outactors (`GameplayStatics.GetAllActorsOfClass` "/CharismaPlugNPlay/Blueprint/Actors/BP_CharismaNPC_Female.BP_CharismaNPC_Female_C"))
      (for _array_element _outactors
        (bind _returnvalue (`|CreateWidget` "/CharismaPlugNPlay/UI/W_Textbox.W_Textbox_C" (`GameplayStatics.GetPlayerController` 0)))
        (`BlueprintMapLibrary.Map_Add` (`self.TextboxMap`) (`/CharismaPlugNPlay/Blueprint/Actors/BP_CharismaNPC_Female.TextBoxTransform` _array_element) _returnvalue)
        (`UserWidget.AddToViewport` _returnvalue 0)
        (`Widget.SetVisibility` _returnvalue "Hidden")))
    (:`then_1`
      ;[1 1 1] Add helper C++ component for adjust positions of UMG items
      (bind _returnvalue_2 (`|AddComponentByClass` "/Script/CharismaPlugNPlay.CharismaTextboxHelper"))
      (bind _output_get (set `self.Helper` _returnvalue_2))
      (bind _keys (`BlueprintMapLibrary.Map_Keys` _textboxmap))
      (bind _values (`BlueprintMapLibrary.Map_Values` _textboxmap))
      (set `CharismaTextboxHelper.Positions` _keys _output_get)
      (set `CharismaTextboxHelper.Widgets` _values _output_get))))

(event `self.ReceiveTick`
  (params (DeltaSeconds :type "Float (single-precision)"))
  (bind _textboxmap (`self.TextboxMap`))
  (bind (_x _y) (`KismetMathLibrary.BreakVector2D` (`WidgetLayoutLibrary.GetViewportSize`)))
  (`|ExecutionSequence`
    (:`then_0`
      ;[1 1 1] Update textboxes to render based on message body and duration
      (bind _keys (`BlueprintMapLibrary.Map_Keys` _textboxmap))
      (for _array_element _keys
        (bind _value (`BlueprintMapLibrary.Map_Find` _textboxmap _array_element))
        (`TextBlock.SetText` (`/CharismaPlugNPlay/UI/W_Textbox.ActorName` _value) (`KismetTextLibrary.Conv_StringToText` (`/CharismaPlugNPlay/Blueprint/Textbox/BP_TextBoxTransform.ActorName` _array_element)))
        (bind (_x_2 _y_2) (`KismetMathLibrary.BreakVector2D` (* (`WidgetLayoutLibrary.ProjectWorldLocationToWidgetPosition` (`GameplayStatics.GetPlayerController` 0) (`SceneComponent.K2_GetComponentLocation` _array_element)) (`WidgetLayoutLibrary.GetViewportScale`))))
        (`/CharismaPlugNPlay/UI/W_Textbox.SetOnScreen` _value (not (or (< _x_2 0.0) (> _x_2 _x) (< _y_2 0.0) (> _y_2 _y))))
        (if (> (`/CharismaPlugNPlay/Blueprint/Textbox/BP_TextBoxTransform.Duration` _array_element) 0.0)
          (`TextBlock.SetText` (`/CharismaPlugNPlay/UI/W_Textbox.SpeechText` _value) (`KismetTextLibrary.Conv_StringToText` (`/CharismaPlugNPlay/Blueprint/Textbox/BP_TextBoxTransform.Message` _array_element)))
          (`Widget.SetVisibility` _value "Visible")
          (set `/CharismaPlugNPlay/Blueprint/Textbox/BP_TextBoxTransform.Duration` (- (`/CharismaPlugNPlay/Blueprint/Textbox/BP_TextBoxTransform.Duration` _array_element) DeltaSeconds) _array_element)
          (else
            (`Widget.SetVisibility` _value "Hidden")))))
    (:`then_1`
      ;[1 1 1] Update textbox positioning on screen
      (`CharismaTextboxHelper.UpdateTextboxesOnScreen` (`self.Helper`)))))

(fn `UserConstructionScript`)