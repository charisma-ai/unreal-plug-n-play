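; Example game mode that runs a Charisma Plug-N-Play playthrough, wiring the player, scene entities and speech recognition to the playthrough instance.
; Each incoming message drives metadata function objects and the player's tap-to-continue.
; Optional save system stores memories and "move-to" character positions, teleporting NPCs on load.
; The first message replays saved memories, polls until all calls return, then sends "StateReady"; EndPlay wipes saves lacking valid state.
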(event `self.ReceiveBeginPlay`
  (bind _playthroughdata (`self.PlaythroughData`))
  (bind _charismaplaythroughinstance (`self.CharismaPlaythroughInstance`))
  ;[1 1 1] Example for initialising a PnP Playthrough
  (bind _returnvalue (`|GenericCreateObject` "/Script/CharismaPlugNPlay.CharismaPlaythroughData"))
  (bind _output_get (set `self.PlaythroughData` _returnvalue))
  (`CharismaPlaythroughData.CollateAllCharismaEntities` _output_get (`self.MetaFunctionClasses`))
  ;;[0 1 0] Check using state system - set state to initialised if true
  (if (`self.UseStateSaveSystem`)
    ;;[0.009721 1 0] Load saved state
    (`self.LoadLocalState`)
    (else
      (set `self.IsStateInitialised` true)))
  (`CharismaPlaythroughInstance.Initialise` (`self.CharismaPlaythroughInstance`) (`self.Connection Params`) (`self.Speech Audio Format`))
  (set `CharismaPlaythroughInstance.CharismaPlayer` (`CharismaPlaythroughData.PlayerComponent` _playthroughdata) _charismaplaythroughinstance)
  (set `CharismaPlaythroughInstance.CharismaEntities` (`CharismaPlaythroughData.Entities` _playthroughdata) _charismaplaythroughinstance)
  (`CharismaPlaythroughInstance.StartPlaythrough` _charismaplaythroughinstance)
  (add `CharismaPlaythroughInstance.OnPlaythroughMessageReceived` _charismaplaythroughinstance (delegate `ParseMessage`)))

(event `SetMemory`
  (params (RecallValue :type String) (SaveValue :type String))
  ;[1 1 1] SetMemory through direct CharismaAPI call - latent event
  (`SetMemory.SetMemory` (`CharismaPlaythroughInstance.PlaythroughToken` (`self.CharismaPlaythroughInstance`)) RecallValue SaveValue))

(event `ParseMessage`
  (params (messageEvent :type "CharismaMessageEvent Structure (by ref)"))
  (bind (_conversationuuid _type _message _endstory _taptocontinue _emotions _memories) (break `CharismaMessageEvent` messageEvent))
  (bind _savedstate (`self.SavedState`))
  (bind (_text _metadata) (break `CharismaMessage` _message))
  (bind _memories_2 (`/CharismaPlugNPlay/Blueprint/SaveGame/SavedCharismaGame.Memories` _savedstate))
  ;[1 1 1] Message handling
  (if (not (`self.IsStateInitialised`))
    ;[0 1 0 0.5] Trigger SetMemory calls for all memories in the saved state
    (`/CharismaPlugNPlay/Blueprint/SaveGame/SavedCharismaGame.LogAllData` _savedstate "SENDING SAVED STATE")
    (bind _keys (`BlueprintMapLibrary.Map_Keys` _memories_2))
    (set `self.MemoriesToLoad` (`KismetArrayLibrary.Array_Length` _keys))
    (for _array_element _keys
      (`SetMemory.SetMemory` (`CharismaPlaythroughInstance.PlaythroughToken` (`self.CharismaPlaythroughInstance`)) _array_element (`BlueprintMapLibrary.Map_Find` _memories_2 _array_element)
        (:`Success`
          _)
        (:`Failure`
          _))
      (set `self.MemoriesLoaded` (+ (`self.MemoriesLoaded`) 1)))
    ;[1 1 1 0.5] Waiting for memories to be set in the playthrough loop
    (if (== (`self.MemoriesToLoad`) (`self.MemoriesLoaded`)) :!label _label
      ;[0.02956 1 0] First message - Send action to start playthrough after memories are loaded
      (`CharismaPlaythroughInstance.SendAction` (`self.CharismaPlaythroughInstance`) "StateReady")
      (set `self.IsStateInitialised` true)
      (else
        (`KismetSystemLibrary.Delay` 0.5)
        (`KismetSystemLibrary.PrintString` (`KismetStringLibrary.Concat_StrStr` "Memories to load: " (`KismetStringLibrary.Conv_IntToString` (`self.MemoriesToLoad`))))
        (`KismetSystemLibrary.PrintString` (`KismetStringLibrary.Concat_StrStr` "Memories loaded: " (`KismetStringLibrary.Conv_IntToString` (`self.MemoriesLoaded`))))
        (goto _label))))
  ;;[0.02956 1 0] Save memory state
  (`self.SaveLocalState` _memories _metadata)
  ;;[1 1 1] Handle metadata
  (`self.HandleMetadata` _metadata)
  ;;[1 1 1] Tap to continue
  (bind _asbp_charisma_player_character (cast `/CharismaPlugNPlay/Blueprint/Player/BP_CharismaPlayerCharacter` (`CharismaPlaythroughData.Player` (`self.PlaythroughData`))))
  (`/CharismaPlugNPlay/Blueprint/Player/BP_CharismaPlayerCharacter.SetPlayerTap` _asbp_charisma_player_character _taptocontinue))

(event `self.ReceiveEndPlay`
  (params (EndPlayReason :type "EEndPlayReason Enum" :default "Destroyed"))
  ;[0.02956 1 0 0.502] Check playthrough state and validate on shutdown
  (if (`self.UseStateSaveSystem`)
    (`self.ValidateLocalState`)))

(fn `EndPlaythrough`
  (`CharismaPlaythroughInstance.EndPlaythrough` (`self.CharismaPlaythroughInstance`)))

(fn `HandleMetadata`
  (params (Metadata :type "Map of String to String"))
  (for _array_element (`CharismaPlaythroughData.MetaDataFunctions` (`self.PlaythroughData`))
    (bind (_value _returnvalue) (`BlueprintMapLibrary.Map_Find` Metadata (`KismetStringLibrary.Conv_NameToString` (`/CharismaPlugNPlay/Blueprint/Metadata/BP_MetadataFunctionBase.MetadataID` _array_element))))
    (if _returnvalue
      (`MetaDataFunctionBase.Execute` _array_element _value (`self.PlaythroughData`)))))

(fn `LoadLocalState`
  (locals (TargetActor :type "/CharismaPlugNPlay/Blueprint/Actors/BP_CharismaNPC_Female Object Reference"))
  (bind _targetactor (`local.TargetActor`))
  (bind _entities (`CharismaPlaythroughData.Entities` (`self.PlaythroughData`)))
  ;[1 1 1] Check if we are using the state save system
  (if (`self.UseStateSaveSystem`)
    (bind _returnvalue (`GameplayStatics.DoesSaveGameExist` "default"))
    (if (not _returnvalue)
      ;[1 1 1 0.5] No save game object present - create a new one
      (bind _returnvalue_2 (`GameplayStatics.CreateSaveGameObject` "/CharismaPlugNPlay/Blueprint/SaveGame/SavedCharismaGame.SavedCharismaGame_C"))
      (`GameplayStatics.SaveGameToSlot` _returnvalue_2 "default"))
    (bind _returnvalue_3 (`GameplayStatics.LoadGameFromSlot` "default"))
    (bind _assaved_charisma_game (cast `/CharismaPlugNPlay/Blueprint/SaveGame/SavedCharismaGame` _returnvalue_3))
    (bind _output_get (set `self.SavedState` _assaved_charisma_game))
    ;[1 1 1 0.5] Loop over all characters - teleport them to correct positions
    (bind (_keypin _valuepin) (`|MapForEach` (`/CharismaPlugNPlay/Blueprint/SaveGame/SavedCharismaGame.CharacterPositions` _output_get))
      (:`then`
        ;[1 1 1] Find target actor
        (for _array_element _entities
          (if (== (`CharismaEntityComponent.EntityId` _array_element) _keypin)
            (bind _asbp_charisma_npc_female (cast `/CharismaPlugNPlay/Blueprint/Actors/BP_CharismaNPC_Female` (`ActorComponent.GetOwner` _array_element)))
            (set `local.TargetActor` _asbp_charisma_npc_female)
            (break)))
        (if (`KismetSystemLibrary.IsValid` (`local.TargetActor`))
          ;[1 1 1] Teleport to destination
          (for _array_element_2 _entities
            (if (== _valuepin (`CharismaEntityComponent.EntityId` _array_element_2))
              (bind _returnvalue_4 (`ActorComponent.GetOwner` _array_element_2))
              (`self.K2_TeleportTo` :`self` _targetactor :`DestLocation` (`self.K2_GetActorLocation` _returnvalue_4))
              (`self.K2_SetActorRotation` _targetactor (`self.K2_GetActorRotation` _returnvalue_4) false)))))
      (:`CompletedPin`
        (return)))
    (else
      (return))))

(fn `SaveLocalState`
  (params (Memories :type "Array of CharismaMemory Structure") (MetaData :type "Map of String to String (by ref)"))
  (locals (HasStateMemory :type Boolean))
  (bind (_value _returnvalue) (`BlueprintMapLibrary.Map_Find` MetaData "move-to"))
  (bind (_lefts _rights) (`KismetStringLibrary.Split` _value ","))
  ;[1 1 1] Check if we are using the state save system
  (if (`self.UseStateSaveSystem`)
    (`KismetSystemLibrary.PrintString` "SAVING LOCAL STATE")
    (for _array_element Memories
      (bind (_recallvalue _savevalue) (break `CharismaMemory` _array_element))
      ;[1 1 1 0.5] Add every memory in SavedState
      (`BlueprintMapLibrary.Map_Add` (`/CharismaPlugNPlay/Blueprint/SaveGame/SavedCharismaGame.Memories` (`self.SavedState`)) _recallvalue _savevalue))
    (if _returnvalue
      ;[1 1 1] Add move-to metadata to save the most up-to-date character positions, if any were passed this message
      (`BlueprintMapLibrary.Map_Add` (`/CharismaPlugNPlay/Blueprint/SaveGame/SavedCharismaGame.CharacterPositions` (`self.SavedState`)) _lefts _rights)
      (`KismetSystemLibrary.PrintString` (`KismetStringLibrary.Concat_StrStr` "Saved character pos: " _lefts)))
    ;[1 1 1 0.5] Save updated state
    (`GameplayStatics.SaveGameToSlot` (`self.SavedState`) "default"))
  (return))

(fn `SendTap`
  (`CharismaPlaythroughInstance.SendTap` (`self.CharismaPlaythroughInstance`)))

(fn `Set Action`
  (params (Action :type String))
  (`CharismaPlaythroughInstance.SendAction` (`self.CharismaPlaythroughInstance`) Action))

(fn `StartSpeechRecognition`
  (returns (Result :type Boolean))
  (bind _bwassuccessful (`CharismaPlaythroughInstance.StartSpeechRecognition` (`self.CharismaPlaythroughInstance`) "Deepgram" "en-US" 16000))
  (return _bwassuccessful))

(fn `StopSpeechRecognition`
  (`CharismaPlaythroughInstance.StopSpeechRecognition` (`self.CharismaPlaythroughInstance`))
  (return))

(fn `UserConstructionScript`
  (locals (ActorArray :type "Array of Object Object Reference") (Entities :type "Array of Object Object Reference")))

(fn `ValidateLocalState`
  (bind _savedstate (`self.SavedState`))
  (bind _memories (`/CharismaPlugNPlay/Blueprint/SaveGame/SavedCharismaGame.Memories` _savedstate))
  (if (`BlueprintMapLibrary.Map_Contains` _memories "state")
    (if (`KismetStringLibrary.EqualEqual_StrStr` (`BlueprintMapLibrary.Map_Find` _memories "state") "NoState")
      (`BlueprintMapLibrary.Map_Clear` _memories :!label _label)
      (`BlueprintMapLibrary.Map_Clear` (`/CharismaPlugNPlay/Blueprint/SaveGame/SavedCharismaGame.CharacterPositions` _savedstate))
      (`GameplayStatics.SaveGameToSlot` (`self.SavedState`) "default"))
    (else
      (goto _label))))

(fn `WipeLocalState`
  (bind _savedstate (`self.SavedState`))
  (`BlueprintMapLibrary.Map_Clear` (`/CharismaPlugNPlay/Blueprint/SaveGame/SavedCharismaGame.Memories` _savedstate))
  (`BlueprintMapLibrary.Map_Clear` (`/CharismaPlugNPlay/Blueprint/SaveGame/SavedCharismaGame.CharacterPositions` _savedstate))
  (`GameplayStatics.SaveGameToSlot` _savedstate "default"))