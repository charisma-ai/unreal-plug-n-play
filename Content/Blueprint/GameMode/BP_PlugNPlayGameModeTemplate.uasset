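; Template game mode that sets up and runs a Charisma Plug-N-Play playthrough on BeginPlay.
; It gathers the player component and entity components from NPC, interactable and move-to actors, then passes them to the playthrough instance.
; Metadata function objects are constructed from a class list and executed when incoming message metadata matches their ID.
; Wrapper functions expose speech recognition, action sending and ending the playthrough.
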(event `self.ReceiveBeginPlay`
  (bind _charismaplaythroughinstance (`self.CharismaPlaythroughInstance`))
  ;[1 1 1] Example for initialising a PnP Playthrough
  (`CharismaPlaythroughInstance.Initialise` (`self.CharismaPlaythroughInstance`) (`self.ConnectionParams`) (`self.Speech Audio Format`))
  (`self.CollateAllCharismaEntities`)
  (set `CharismaPlaythroughInstance.CharismaPlayer` (`self.Player`) (`self.CharismaPlaythroughInstance`))
  (set `CharismaPlaythroughInstance.CharismaEntities` (`self.BaseEntities`) (`self.CharismaPlaythroughInstance`))
  (`CharismaPlaythroughInstance.StartPlaythrough` _charismaplaythroughinstance)
  (add `CharismaPlaythroughInstance.OnPlaythroughMessageReceived` _charismaplaythroughinstance (delegate `ParseMessageForMetadata`)))

(event `ParseMessageForMetadata`
  (params (messageEvent :type "CharismaMessageEvent Structure (by ref)"))
  ;[1 1 1] Metadata handling
  (for _array_element (`self.MetadataFunctions`)
    (bind (_value _returnvalue) (`BlueprintMapLibrary.Map_Find` (`.Metadata` (break `CharismaMessage` (`.Message` (break `CharismaMessageEvent` messageEvent)))) (`KismetStringLibrary.Conv_NameToString` (`/CharismaPlugNPlay/Blueprint/Metadata/BP_MetadataFunction.MetadataID` _array_element))))
    (if _returnvalue
      (`/CharismaPlugNPlay/Blueprint/Metadata/BP_MetadataFunction.Execute` _array_element _value))))

(fn `CollectAllCharismaEntities`
  (locals (ActorEntities :type "Array of CharismaPnPActorComponent Object Reference") (SimpleEntities :type "Array of CharismaEntityComponent Object Reference"))
  (bind _simpleentities (`local.SimpleEntities`))
  ;[1 1 1] Collect Charisma entities and register to Metadata Functions
  (`|ExecutionSequence`
    (:`then_0`
      (bind _returnvalue (`GameplayStatics.GetActorOfClass` "/CharismaPlugNPlay/Blueprint/Player/BP_CharismaPlayerCharacter.BP_CharismaPlayerCharacter_C"))
      (set `self.Player` (`self.GetComponentByClass` _returnvalue "/Script/CharismaPlugNPlay.CharismaPlayerComponent")))
    (:`then_1`
      (bind _outactors (`GameplayStatics.GetAllActorsOfClass` "/CharismaPlugNPlay/Blueprint/Actors/BP_CharismaNPC_Female.BP_CharismaNPC_Female_C"))
      (for _array_element _outactors
        (`KismetArrayLibrary.Array_Add` (`local.SimpleEntities`) (`self.GetComponentByClass` _array_element "/Script/CharismaPlugNPlay.CharismaEntityComponent"))))
    (:`then_2`
      (bind _outactors_2 (`GameplayStatics.GetAllActorsOfClass` "/CharismaPlugNPlay/Blueprint/Actors/Entities/BP_CharismaInteractableTemplate.BP_CharismaInteractableTemplate_C"))
      (for _array_element_2 _outactors_2
        (`KismetArrayLibrary.Array_Add` _simpleentities (`self.GetComponentByClass` _array_element_2 "/Script/CharismaPlugNPlay.CharismaEntityComponent"))))
    (:`then_3`
      (bind _outactors_3 (`GameplayStatics.GetAllActorsOfClass` "/CharismaPlugNPlay/Blueprint/Actors/Entities/BP_CharismaMoveTo.BP_CharismaMoveTo_C"))
      (for _array_element_3 _outactors_3
        (`KismetArrayLibrary.Array_Add` _simpleentities (`self.GetComponentByClass` _array_element_3 "/Script/CharismaPlugNPlay.CharismaEntityComponent"))))
    (:`then_4`
      (set `self.BaseEntities` (`local.SimpleEntities`)))
    (:`then_5`
      (for _array_element_4 (`self.MetadataClasses`)
        (bind _returnvalue_2 (`|GenericCreateObject` _array_element_4))
        (`KismetArrayLibrary.Array_Add` (`self.MetadataFunctions`) _returnvalue_2)
        (set `/CharismaPlugNPlay/Blueprint/Metadata/BP_MetadataFunction.PlaythroughEntities` (make `/CharismaPlugNPlay/Blueprint/BP_Struct_PlaythroughEntities` _returnvalue _simpleentities) _returnvalue_2)))))

(fn `EndPlaythrough`
  (`CharismaPlaythroughInstance.EndPlaythrough` (`self.CharismaPlaythroughInstance`)))

(fn `Set Action`
  (params (Action :type String))
  (`CharismaPlaythroughInstance.SendAction` (`self.CharismaPlaythroughInstance`) Action))

(fn `StartSpeechRecognition`
  (returns (Result :type Boolean))
  (bind _bwassuccessful (`CharismaPlaythroughInstance.StartSpeechRecognition` (`self.CharismaPlaythroughInstance`) "AWS" "en-US" "pcm" 16000))
  (return _bwassuccessful))

(fn `StopSpeechRecognition`
  (`CharismaPlaythroughInstance.StopSpeechRecognition` (`self.CharismaPlaythroughInstance`))
  (return))

(fn `UserConstructionScript`
  (locals (ActorArray :type "Array of Object Object Reference") (Entities :type "Array of Object Object Reference")))