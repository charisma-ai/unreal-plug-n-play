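; Charisma metadata function Blueprint that plays a named animation on an NPC during a playthrough.
; Execute splits the comma-separated metadata into an entity ID and animation name, then searches the playthrough's entities for the matching ID.
; The matched entity's owner is cast to BP_CharismaNPC_Female, so only that class is supported, and receives a RequestAnimation call with the name.
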(fn `Execute`
  (params (metaData :type String) (playthroughData :type "CharismaPlaythroughData Object Reference"))
  (locals (TargetActor :type "/CharismaPlugNPlay/Blueprint/Actors/BP_CharismaNPC_Female Object Reference"))
  (bind (_lefts _rights _returnvalue) (`KismetStringLibrary.Split` metaData ","))
  (bind _targetactor (`local.TargetActor`))
  ;[1 1 1] Find Target Actor, and request animation by name.
  (if _returnvalue
    (for _array_element (`CharismaPlaythroughData.Entities` playthroughData)
      (if (== (`CharismaEntityComponent.EntityId` _array_element) _lefts)
        (bind _asbp_charisma_npc_female (cast `/CharismaPlugNPlay/Blueprint/Actors/BP_CharismaNPC_Female` (`ActorComponent.GetOwner` _array_element)))
        (set `local.TargetActor` _asbp_charisma_npc_female)
        (break)))
    (if (`KismetSystemLibrary.IsValid` _targetactor)
      (`/CharismaPlugNPlay/Blueprint/Actors/BP_CharismaNPC_Female.RequestAnimation` _targetactor _rights))))