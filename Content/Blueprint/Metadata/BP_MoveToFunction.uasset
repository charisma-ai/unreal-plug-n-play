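; Charisma metadata function that sends an NPC to a destination entity in the playthrough.
; Execute splits the metadata string at a comma into a mover ID and a destination ID, matching each against the playthrough's entity IDs.
; The mover's owner must cast to BP_CharismaNPC_Female, which then receives the destination's owner through SetMoveToTarget.
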(fn `Execute`
  (params (metaData :type String) (playthroughEntities :type "CharismaPlaythroughEntities Structure (by ref)"))
  (locals (TargetActor :type "/CharismaPlugNPlay/Blueprint/Actors/BP_CharismaNPC_Female Object Reference"))
  (bind (_player _entities) (break `CharismaPlaythroughEntities` playthroughEntities))
  (bind (_lefts _rights _returnvalue) (`KismetStringLibrary.Split` metaData ","))
  (if _returnvalue
    ;[1 1 1] Find target actor
    (for _array_element _entities
      (if (== (`CharismaEntityComponent.EntityId` _array_element) _lefts)
        (bind _asbp_charisma_npc_female (cast `/CharismaPlugNPlay/Blueprint/Actors/BP_CharismaNPC_Female` (`ActorComponent.GetOwner` _array_element)))
        (set `local.TargetActor` _asbp_charisma_npc_female)
        (break)))
    (if (`KismetSystemLibrary.IsValid` (`local.TargetActor`))
      ;[1 1 1] Find target destination
      (for _array_element_2 _entities
        (if (== _rights (`CharismaEntityComponent.EntityId` _array_element_2))
          (`/CharismaPlugNPlay/Blueprint/Actors/BP_CharismaNPC_Female.SetMoveToTarget` (`local.TargetActor`) (`ActorComponent.GetOwner` _array_element_2))
          (return))))))