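; Charisma metadata function that sets which entity an NPC looks at during a playthrough.
; It splits the value on a comma, matches the left ID to a BP_CharismaNPC_Female among the playthrough entities, then passes the owner of the right ID's entity to SetLookAtTarget.
; A comma-less "player" value targets the player on the existing TargetActor, without looking one up or checking validity.
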(fn `Execute`
  (params (MetadataValue :type String))
  (locals (TargetActor :type "/CharismaPlugNPlay/Blueprint/Actors/BP_CharismaNPC_Female Object Reference"))
  (bind (_lefts _rights _returnvalue) (`KismetStringLibrary.Split` MetadataValue ","))
  (bind (_player _entities) (break `/CharismaPlugNPlay/Blueprint/BP_Struct_PlaythroughEntities` (`self.PlaythroughEntities`)))
  ;[1 1 1] Find Actor
  (if _returnvalue
    (for _array_element _entities
      (if (== (`CharismaEntityComponent.EntityId` _array_element) _lefts)
        (bind _asbp_charisma_npc_female (cast `/CharismaPlugNPlay/Blueprint/Actors/BP_CharismaNPC_Female` (`ActorComponent.GetOwner` _array_element)))
        (set `local.TargetActor` _asbp_charisma_npc_female)
        (break)))
    ;[1 1 1] Find look at target and send it to the Actor
    (if (`KismetSystemLibrary.IsValid` (`local.TargetActor`))
      (for _array_element_2 _entities
        (if (== _rights (`CharismaEntityComponent.EntityId` _array_element_2))
          (`/CharismaPlugNPlay/Blueprint/Actors/BP_CharismaNPC_Female.SetLookAtTarget` (`local.TargetActor`) (`ActorComponent.GetOwner` _array_element_2))
          (return))))
    (elif (== MetadataValue "player")
      (`/CharismaPlugNPlay/Blueprint/Actors/BP_CharismaNPC_Female.SetLookAtTarget` (`local.TargetActor`) _player)
      (return))))