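; SavedCharismaGame is a save-game Blueprint for Charisma data, holding a Memories map and a CharacterPositions map.
; LogAllData prints a given preface, then each memory key and value as a "SAVED DATA" debug string.
; The character-position loop is nested inside the memory loop, so every position reprints per memory and none print when Memories is empty.
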(fn `LogAllData`
  (params (Preface :type String))
  (bind _characterpositions (`self.CharacterPositions`))
  (bind _memories (`self.Memories`))
  (`KismetSystemLibrary.PrintString` null Preface)
  (bind _keys (`BlueprintMapLibrary.Map_Keys` _memories))
  (for _array_element _keys
    (`KismetSystemLibrary.PrintString` null (`KismetStringLibrary.Concat_StrStr` "SAVED DATA: Memory: " (`KismetStringLibrary.Concat_StrStr` (`KismetStringLibrary.Concat_StrStr` _array_element "  ") (`BlueprintMapLibrary.Map_Find` _memories _array_element))))
    (bind _keys_2 (`BlueprintMapLibrary.Map_Keys` _characterpositions))
    (for _array_element_2 _keys_2
      (`KismetSystemLibrary.PrintString` null (`KismetStringLibrary.Concat_StrStr` "SAVED DATA: Character pos: " (`KismetStringLibrary.Concat_StrStr` (`KismetStringLibrary.Concat_StrStr` _array_element_2 "  ") (`BlueprintMapLibrary.Map_Find` _characterpositions _array_element_2)))))))