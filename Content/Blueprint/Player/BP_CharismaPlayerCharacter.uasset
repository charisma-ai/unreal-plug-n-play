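; Player character for a Charisma story experience, handling movement, interaction, typed or spoken replies, tap-to-continue and session restart or shutdown.
; Tick picks the first unused online interactable within view angle and range, from actors cached in the construction script, and toggles its prompt.
; Replies from the reply widget go to CharismaPlayer, whose speech transcripts update that widget.
; BP_PlugNPlayGameMode handles speech recognition, taps, playthrough end and local state.
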(event `self.ReceiveBeginPlay`
  ;[1 1 1] Input mapping
  (bind _asplayer_controller (cast `PlayerController` (`self.GetController`)))
  (bind _returnvalue (pcsubsystem `EnhancedInputLocalPlayerSubsystem` _asplayer_controller))
  (`/Engine/EditorBlueprintResources/StandardMacros.IsValid` _returnvalue
    (:`Is Valid`
      (`EnhancedInputSubsystemInterface.AddMappingContext` _returnvalue "/CharismaPlugNPlay/Inputs/IMP_CharismaPlayer.IMP_CharismaPlayer" 0 (struct))
      (bind _asbp_plug_nplay_game_mode (cast `/CharismaPlugNPlay/Blueprint/GameMode/BP_PlugNPlayGameMode` (`GameplayStatics.GetGameMode`)))
      (set `self.GameMode` _asbp_plug_nplay_game_mode)
      (bind _returnvalue_2 (`|CreateWidget` "/CharismaPlugNPlay/UI/W_PlayerReplyUI.W_PlayerReplyUI_C"))
      (bind _output_get (set `self.ReplyUI` _returnvalue_2))
      (add `/CharismaPlugNPlay/UI/W_PlayerReplyUI.OnResultReply` _output_get (delegate `ParseReply`))
      (`WidgetBlueprintLibrary.SetInputMode_GameOnly` (`GameplayStatics.GetPlayerController` 0))
      (bind _returnvalue_3 (`|CreateWidget` "/CharismaPlugNPlay/UI/W_FadeScreen.W_FadeScreen_C"))
      (bind _output_get_2 (set `self.FadeScreenUI` _returnvalue_3))
      (`UserWidget.AddToViewport` _output_get_2 0)
      (bind _returnvalue_4 (`|CreateWidget` "/CharismaPlugNPlay/UI/W_TapContinueUI.W_TapContinueUI_C"))
      (bind _output_get_3 (set `self.TapContinueUI` _returnvalue_4))
      (`UserWidget.AddToViewport` _output_get_3 0)
      (`Widget.SetVisibility` (`self.TapContinueUI`) "Hidden")
      (add `CharismaPlayerComponent.OnSpeechRecognition` (`self.CharismaPlayer`) (delegate `Speech Recognition result`)))))

(event `EnhancedInput|/CharismaPlugNPlay/Inputs/IA_Look`
  (params (ActionValue :type "Vector2D Structure") (ElapsedSeconds :type "Float (double-precision)") (TriggeredSeconds :type "Float (double-precision)") (InputAction :type "InputAction Object Reference" :default "/CharismaPlugNPlay/Inputs/IA_Look.IA_Look"))
  ;[1 1 1] Looking
  (:`Triggered`
    (`self.AddControllerYawInput` ActionValue_X)
    (`self.AddControllerPitchInput` ActionValue_Y)))

(event `ParseReply`
  (params (ResultReply :type String))
  ;[1 1 1] Finalize reply event
  (`CharismaPlayerComponent.OnReply` (`self.CharismaPlayer`) ResultReply)
  (set `self.IsReplying` false))

(event `Speech Recognition result`
  (params (Transcript :type String) (IsFinal :type Boolean))
  ;[1 1 1] Parse speech result
  (`self.SetSpeechResult` Transcript IsFinal))

(event `EnhancedInput|/CharismaPlugNPlay/Inputs/IA_Submit`
  (params (ActionValue :type Boolean) (ElapsedSeconds :type "Float (double-precision)") (TriggeredSeconds :type "Float (double-precision)") (InputAction :type "InputAction Object Reference" :default "/CharismaPlugNPlay/Inputs/IA_Submit.IA_Submit"))
  ;[1 1 1] Replying events
  (:`Started`
    (if (`self.IsReplying`)
      (`/CharismaPlugNPlay/UI/W_PlayerReplyUI.OnSubmitText` (`self.ReplyUI`)))))

(event `EnhancedInput|/CharismaPlugNPlay/Inputs/IA_Move`
  (params (ActionValue :type "Vector2D Structure") (ElapsedSeconds :type "Float (double-precision)") (TriggeredSeconds :type "Float (double-precision)") (InputAction :type "InputAction Object Reference" :default "/CharismaPlugNPlay/Inputs/IA_Move.IA_Move"))
  (bind (_returnvalue_roll _returnvalue_pitch _returnvalue_yaw) (`KismetMathLibrary.BreakRotator` (`self.GetControlRotation`)))
  (bind (_returnvalue_roll_2 _returnvalue_pitch_2 _returnvalue_yaw_2) (`KismetMathLibrary.BreakRotator` (`self.GetControlRotation`)))
  ;[1 1 1] Movement
  (:`Triggered`
    (`self.AddMovementInput` (`KismetMathLibrary.GetRightVector` (`KismetMathLibrary.MakeRotator` _returnvalue_roll 0.0 _returnvalue_yaw)) ActionValue_X)
    (`self.AddMovementInput` (`KismetMathLibrary.GetForwardVector` (`KismetMathLibrary.MakeRotator` 0.0 0.0 _returnvalue_yaw_2)) ActionValue_Y)))

(event `EnhancedInput|/CharismaPlugNPlay/Inputs/IA_Edit`
  (params (ActionValue :type Boolean) (ElapsedSeconds :type "Float (double-precision)") (TriggeredSeconds :type "Float (double-precision)") (InputAction :type "InputAction Object Reference" :default "/CharismaPlugNPlay/Inputs/IA_Edit.IA_Edit"))
  ;[1 1 1] Replying events
  (:`Started`
    (if (`self.IsReplying`)
      (`/CharismaPlugNPlay/UI/W_PlayerReplyUI.SetToTextInput` (`self.ReplyUI`)))))

(event `EnhancedInput|/CharismaPlugNPlay/Inputs/IA_Interact`
  (params (ActionValue :type Boolean) (ElapsedSeconds :type "Float (double-precision)") (TriggeredSeconds :type "Float (double-precision)") (InputAction :type "InputAction Object Reference" :default "/CharismaPlugNPlay/Inputs/IA_Interact.IA_Interact"))
  (bind _currentinteractable (`self.CurrentInteractable`))
  (bind _charismainteractable (`/CharismaPlugNPlay/Blueprint/Actors/Entities/BP_CharismaInteractableTemplate.CharismaInteractable` _currentinteractable))
  ;[1 1 1] Interaction
  (:`Triggered`
    (if (`KismetSystemLibrary.IsValid` _currentinteractable)
      (bind _returnvalue (`CharismaInteractableComponent.HasBeenUsed` _charismainteractable))
      (if (not _returnvalue)
        (`CharismaInteractableComponent.Interact` _charismainteractable)
        (set `/CharismaPlugNPlay/UI/W_Interact.IsPressed` true (`self.InteractUI`))))))

(event `EnhancedInput|/CharismaPlugNPlay/Inputs/IA_Talk`
  (params (ActionValue :type Boolean) (ElapsedSeconds :type "Float (double-precision)") (TriggeredSeconds :type "Float (double-precision)") (InputAction :type "InputAction Object Reference" :default "/CharismaPlugNPlay/Inputs/IA_Talk.IA_Talk"))
  ;[1 1 1] Replying events
  (:`Started`
    (if (`self.IsReplying`)
      (`self.StartSpeak`)
      (`/CharismaPlugNPlay/UI/W_PlayerReplyUI.SetToSpeechInput` (`self.ReplyUI`))))
  (:`Completed`
    (if (`self.IsReplying`)
      (`self.EndSpeak`))))

(event `EnhancedInput|/CharismaPlugNPlay/Inputs/IA_Restart`
  (params (ActionValue :type Boolean) (ElapsedSeconds :type "Float (double-precision)") (TriggeredSeconds :type "Float (double-precision)") (InputAction :type "InputAction Object Reference" :default "/CharismaPlugNPlay/Inputs/IA_Restart.IA_Restart"))
  ;[1 1 1] Restarting
  (:`Triggered`
    (if (`self.Ending`)
      (`/CharismaPlugNPlay/Blueprint/GameMode/BP_PlugNPlayGameMode.EndPlaythrough` (`self.GameMode`))
      (`GameplayStatics.OpenLevel` "None"))))

(event `EnhancedInput|/CharismaPlugNPlay/Inputs/IA_Shutdown`
  (params (ActionValue :type Boolean) (ElapsedSeconds :type "Float (double-precision)") (TriggeredSeconds :type "Float (double-precision)") (InputAction :type "InputAction Object Reference" :default "/CharismaPlugNPlay/Inputs/IA_Shutdown.IA_Shutdown"))
  ;[1 1 1] Shutdown
  (:`Triggered`
    (`/CharismaPlugNPlay/Blueprint/GameMode/BP_PlugNPlayGameMode.ValidateLocalState` (`self.GameMode`))
    (`KismetSystemLibrary.QuitGame` null "Quit")))

(event `EnhancedInput|/CharismaPlugNPlay/Inputs/IA_ShutdownWipeData`
  (params (ActionValue :type Boolean) (ElapsedSeconds :type "Float (double-precision)") (TriggeredSeconds :type "Float (double-precision)") (InputAction :type "InputAction Object Reference" :default "/CharismaPlugNPlay/Inputs/IA_ShutdownWipeData.IA_ShutdownWipeData"))
  ;[1 1 1] Shutdown with local data wipe
  (:`Triggered`
    (`/CharismaPlugNPlay/Blueprint/GameMode/BP_PlugNPlayGameMode.WipeLocalState` (`self.GameMode`))
    (`KismetSystemLibrary.QuitGame` null "Quit")))

(event `EnhancedInput|/CharismaPlugNPlay/Inputs/IA_TapContinue`
  (params (ActionValue :type Boolean) (ElapsedSeconds :type "Float (double-precision)") (TriggeredSeconds :type "Float (double-precision)") (InputAction :type "InputAction Object Reference" :default "/CharismaPlugNPlay/Inputs/IA_TapContinue.IA_TapContinue"))
  ;[1 1 1] Tap continue
  (:`Triggered`
    (if (`self.IsShowingTapToContinue`)
      (`/CharismaPlugNPlay/Blueprint/GameMode/BP_PlugNPlayGameMode.SendTap` (`self.GameMode`))
      (`self.SetPlayerTap` false))))

(event `self.ReceiveTick`
  (params (DeltaSeconds :type "Float (single-precision)"))
  (bind _returnvalue (`SceneComponent.K2_GetComponentLocation` (`self.Camera`)))
  ;[1 1 1] Detect Interactable
  (if (`self.Ending`)
    _
    (elif (not (`self.IsReplying`))
      (set `self.CurrentInteractable` null)
      (for _array_element (`self.InteractableArray`)
        (bind _charismainteractable (`/CharismaPlugNPlay/Blueprint/Actors/Entities/BP_CharismaInteractableTemplate.CharismaInteractable` _array_element))
        (if (`CharismaEntityComponent.IsOnline` _charismainteractable)
          (bind _returnvalue_2 (`self.K2_GetActorLocation` _array_element))
          (if (< (`self.GetAngleBetweenTwoVectors` (- _returnvalue_2 _returnvalue) (`SceneComponent.GetForwardVector` (`self.Camera`))) 15.0)
            (if (< (`KismetMathLibrary.Vector_Distance` _returnvalue _returnvalue_2) 250.0)
              (bind _returnvalue_3 (`CharismaInteractableComponent.HasBeenUsed` _charismainteractable))
              (if (not _returnvalue_3)
                (set `self.CurrentInteractable` _array_element)
                (break))))))
      (`self.SetInteractPromptVisible` (`KismetSystemLibrary.IsValid` (`self.CurrentInteractable`))))))

(fn `EndPlayerSession`
  (`/CharismaPlugNPlay/UI/W_FadeScreen.Fade` (`self.FadeScreenUI`))
  (set `self.Ending` true))

(fn `EndSpeak`
  (`/CharismaPlugNPlay/Blueprint/GameMode/BP_PlugNPlayGameMode.StopSpeechRecognition` (`self.GameMode`)))

(fn `GetAngleBetweenTwoVectors`
  (params (VectorA :type "Vector Structure") (VectorB :type "Vector Structure"))
  (returns (Angle :type "Float (double-precision)"))
  (return (`KismetMathLibrary.DegAcos` (`KismetMathLibrary.Dot_VectorVector` (`KismetMathLibrary.Normal` VectorA) (`KismetMathLibrary.Normal` VectorB)))))

(fn `SetInteractPromptVisible`
  (params (visible :type Boolean))
  (bind _interactui (`self.InteractUI`))
  (bind _interactui_2 (`self.InteractUI`))
  (bind _returnvalue (`KismetSystemLibrary.IsValid` _interactui))
  (if visible
    (if (not _returnvalue)
      (bind _returnvalue_2 (`|CreateWidget` "/CharismaPlugNPlay/UI/W_Interact.W_Interact_C"))
      (bind _output_get (set `self.InteractUI` _returnvalue_2)))
    (if (not (`Widget.IsInViewport` _output_get))
      (`UserWidget.AddToViewport` _interactui_2 0)
      (set `/CharismaPlugNPlay/UI/W_Interact.IsPressed` false _interactui_2)
      (`Widget.SetVisibility` _interactui_2 "Visible"))
    (elif _returnvalue
      (`Widget.RemoveFromParent` _interactui))))

(fn `SetPlayerReadyForReply`
  (bind _interactui (`self.InteractUI`))
  (bind _replyui (`self.ReplyUI`))
  (if (not (`self.IsReplying`))
    (if (not (`KismetSystemLibrary.IsValid` _replyui))
      (bind _returnvalue (`|CreateWidget` "/CharismaPlugNPlay/UI/W_PlayerReplyUI.W_PlayerReplyUI_C"))
      (set `self.ReplyUI` _returnvalue))
    (`UserWidget.AddToViewport` _replyui 0)
    (set `self.IsReplying` true)
    (`/CharismaPlugNPlay/UI/W_PlayerReplyUI.SetActive` (`self.ReplyUI`) true)
    (if (`KismetSystemLibrary.IsValid` _interactui)
      (`Widget.SetVisibility` _interactui "Hidden"))
    (else
      (`Widget.RemoveFromParent` _replyui))))

(fn `SetPlayerTap`
  (params (EnableTapUI :type Boolean))
  (bind _tapcontinueui (`self.TapContinueUI`))
  (bind _output_get (set `self.IsShowingTapToContinue` EnableTapUI))
  (if _output_get
    (set `Widget.Visibility` "Visible" _tapcontinueui)
    (else
      (set `Widget.Visibility` "Hidden" _tapcontinueui))))

(fn `SetSpeechResult`
  (params (Transcript :type String) (IsFinal :type Boolean))
  (`/CharismaPlugNPlay/UI/W_PlayerReplyUI.UpdateTextWithSpeech` (`self.ReplyUI`) Transcript))

(fn `StartSpeak`
  (`/CharismaPlugNPlay/Blueprint/GameMode/BP_PlugNPlayGameMode.StartSpeechRecognition` (`self.GameMode`)))

(fn `UserConstructionScript`
  (bind _outactors (`GameplayStatics.GetAllActorsOfClass` "/CharismaPlugNPlay/Blueprint/Actors/Entities/BP_CharismaInteractableTemplate.BP_CharismaInteractableTemplate_C"))
  (set `self.InteractableArray` _outactors))