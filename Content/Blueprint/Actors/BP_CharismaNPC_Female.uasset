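; Female NPC actor for Charisma plug-and-play conversations, reacting to playthrough messages as either the speaker or a spectator.
; As speaker it stores text, speech and emotions and looks at the player; as spectator it looks at whoever is talking.
; Speech bytes import at runtime into a sound wave, also exported to raw PCM for morph-target lipsync.
; ApplyMessage then drives face, animation, text box, audio and behaviour-tree movement, and clears pending state.
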(event `self.ReceiveBeginPlay`
  ;[1 1 1] Initialise
  (`/CharismaPlugNPlay/Blueprint/Animation/BPI_NPCLipsyncInterface.AddLipsyncComponents` (`self.NPCLipsync`) self (`self.Mesh`) (`self.Viseme Morph Targets`))
  (add `CharismaEntityComponent.OnMessage` (`self.CharismaPnPActor`) (delegate `OnMessageReceived`))
  (bind _asbp_plug_nplay_game_mode_template (cast `/CharismaPlugNPlay/Blueprint/GameMode/BP_PlugNPlayGameModeTemplate` (`GameplayStatics.GetGameMode`)))
  (bind _returnvalue (`RuntimeAudioImporterLibrary.CreateRuntimeAudioImporter`))
  (set `self.Audio Importer` _returnvalue)
  (set `self.Audio Format` (`/CharismaPlugNPlay/Blueprint/GameMode/BP_PlugNPlayGameModeTemplate.Audio Format` _asbp_plug_nplay_game_mode_template))
  (bind _asabp_npcfemale (cast `/CharismaPlugNPlay/Animations/ABP_NPCFemale` (`SkeletalMeshComponent.GetAnimInstance` (`self.Mesh`))))
  (set `self.NPCAnimationController` _asabp_npcfemale)
  (`/CharismaPlugNPlay/Blueprint/Textbox/BP_TextBoxTransform.SetActorName` (`self.TextBoxTransform`) (`CharismaEntityComponent.EntityId` (`self.CharismaPnPActor`))))

(event `OnMessageReceived`
  (params (MessageEvent :type "CharismaMessageEvent Structure (by ref)") (isEntityMatch :type Boolean))
  ;[1 1 1] Message Resolution
  (if isEntityMatch
    (`self.InterpretMessageAsReceiver` MessageEvent)
    (else
      (`self.InterpretMessageAsSpectator` MessageEvent))))

(event `OnMessageResolve`
  (bind _audio_importer (`self.Audio Importer`))
  (bind (_audio _duration) (break `CharismaSpeech` (`self.Speech`)))
  ;[1 1 1] Message Resolution
  (if (not (`KismetArrayLibrary.Array_IsEmpty` _audio))
    (add `RuntimeAudioImporterLibrary.OnResult` _audio_importer (delegate `OnAudioImported`))
    (`RuntimeAudioImporterLibrary.ImportAudioFromBuffer` _audio_importer _audio (`self.Audio Format`))
    (set `self.Duration` _duration)
    (set `self.RAWData` _audio)
    (else
      (`self.ApplyMessage` null))))

(event `OnAudioImported`
  (params (Importer :type "RuntimeAudioImporterLibrary Object Reference") (ImportedSoundWave :type "ImportedSoundWave Object Reference") (Status :type "ERuntimeImportStatus Enum" :default "SuccessfulImport"))
  ;[1 1 1] Message Resolution
  (switch `ERuntimeImportStatus` Status
    (:`SuccessfulImport`
      (`RuntimeAudioExporter.ExportSoundWaveToRAWBuffer` ImportedSoundWave "Int16" (`self.Override Options`) (delegate `On Export`))
      (`self.ApplyMessage` ImportedSoundWave))))

(event `On Export`
  (params (bSucceeded :type Boolean) (AudioData :type "Array of Byte (by ref)"))
  ;[1 1 1] Message Resolution
  (`/CharismaPlugNPlay/Blueprint/Animation/BPI_NPCLipsyncInterface.FeedAudio` (`self.NPCLipsync`) AudioData (/ (`self.Duration`) 1000.0)))

(fn `ApplyMessage`
  (params (AudioWave :type "ImportedSoundWave Object Reference"))
  (bind _audio (`self.Audio`))
  (bind _textboxtransform (`self.TextBoxTransform`))
  (bind _look_at_target (`self.Look at Target`))
  (bind _returnvalue (/ (`.Duration` (break `CharismaSpeech` (`self.Speech`))) 1000.0))
  (`|ExecutionSequence`
    (:`then_0`
      ;[1 1 1] Apply emotion to NPC, via facial expressions and animation controller
      (bind (_emotion _intensity) (`self.GetStrongestEmotion`))
      (if (not (`KismetStringLibrary.IsEmpty` _emotion))
        (`/CharismaPlugNPlay/Blueprint/Animation/BP_NPCFacialAnimationComponent.RequestFacialExpression` (`self.NPCFacialAnimationComponent`) _emotion _intensity)
        (`/CharismaPlugNPlay/Animations/ABP_NPCFemale.SetEmotion` (`self.NPCAnimationController`) _emotion _intensity)
        (else
          (`/CharismaPlugNPlay/Animations/ABP_NPCFemale.SetEmotion` (`self.NPCAnimationController`) "" 0.0))))
    (:`then_1`
      ;[1 1 1] Apply look at target
      (if (`KismetSystemLibrary.IsValid` _look_at_target)
        (`/CharismaPlugNPlay/Animations/ABP_NPCFemale.SetLookAt` (`self.NPCAnimationController`) _look_at_target)))
    (:`then_2`
      ;[1 1 1] Apply message and print it in the textbox
      (if (not (`KismetStringLibrary.IsEmpty` (`self.Message`)))
        (set `/CharismaPlugNPlay/Blueprint/Textbox/BP_TextBoxTransform.Duration` (+ _returnvalue 3.0) _textboxtransform)
        (set `/CharismaPlugNPlay/Blueprint/Textbox/BP_TextBoxTransform.Message` (`KismetTextLibrary.Conv_TextToString` (`KismetTextLibrary.Conv_StringToText` (`self.Message`))) _textboxtransform)))
    (:`then_3`
      ;[1 1 1] Apply speech audio
      (`/CharismaPlugNPlay/Animations/ABP_NPCFemale.SetIsTalking` (`self.NPCAnimationController`) _returnvalue)
      (`AudioComponent.SetSound` _audio AudioWave)
      (`AudioComponent.Play` _audio 0.0)
      (`AudioComponent.StopDelayed` _audio _returnvalue))
    (:`then_4`
      ;[1 1 1] Apply move-to target
      (if (`KismetSystemLibrary.IsValid` (`self.MoveToTarget`))
        (`AIController.RunBehaviorTree` (`AIBlueprintHelperLibrary.GetAIController` self) "/CharismaPlugNPlay/Blueprint/Actors/AI/BT_NPC.BT_NPC")
        (`BlackboardComponent.SetValueAsVector` (`AIBlueprintHelperLibrary.GetBlackboard` null) "TargetLocation" (`self.K2_GetActorLocation` (`self.MoveToTarget`)))))
    (:`then_5`
      (`self.ClearAllPending`))))

(fn `ClearAllPending`
  (set `self.AnimationToPlay` "")
  (set `self.MoveToTarget` null)
  (set `self.Look at Target` null)
  (set `self.Speech` (struct))
  (set `self.Message` ""))

(fn `GetStrongestEmotion`
  (returns (Emotion :type String) (Intensity :type "Float (double-precision)"))
  (locals (MaxIntensity :type "Float (double-precision)" :default -1.0) (MaxEmotion :type String))
  (bind _emotionmap (`self.EmotionMap`))
  (if (> (`BlueprintMapLibrary.Map_Length` _emotionmap) 0)
    (bind _keys (`BlueprintMapLibrary.Map_Keys` _emotionmap))
    (for _array_element _keys
      (bind _value (`BlueprintMapLibrary.Map_Find` _emotionmap _array_element))
      (if (> _value (`local.MaxIntensity`))
        (set `local.MaxIntensity` _value)
        (set `local.MaxEmotion` _array_element)))
    (return (`local.MaxEmotion`) (`local.MaxIntensity`))
    (else
      (return "" 0.0))))

(fn `InterpretMessageAsReceiver`
  (params (MessageEvent :type "CharismaMessageEvent Structure"))
  (bind (_conversationuuid _type _message _endstory _taptocontinue _emotions) (break `CharismaMessageEvent` MessageEvent))
  (bind (_text _metadata _character _speech) (break `CharismaMessage` _message))
  ;[1 1 1] Apply text and speech
  (`self.SetMessageBody` _text)
  (`self.SetSpeechData` _speech)
  ;[1 1 1] Look for any emotions associated with the message
  (for _array_element _emotions
    (if (== (`CharismaEntityComponent.EntityId` (`self.CharismaPnPActor`)) (`.Name` (break `CharismaEmotion` _array_element)))
      (`self.Register Active Emotion` _array_element)))
  ;[1 1 1] Look at the player, as we are talking to them
  (bind _asbp_plug_nplay_game_mode_template (cast `/CharismaPlugNPlay/Blueprint/GameMode/BP_PlugNPlayGameModeTemplate` (`GameplayStatics.GetGameMode`)))
  (bind _asbp_charisma_player_character (cast `/CharismaPlugNPlay/Blueprint/Player/BP_CharismaPlayerCharacter` (`ActorComponent.GetOwner` (`CharismaPlaythroughInstance.CharismaPlayer` (`/CharismaPlugNPlay/Blueprint/GameMode/BP_PlugNPlayGameModeTemplate.CharismaPlaythroughInstance` _asbp_plug_nplay_game_mode_template)))))
  (`self.SetLookAtTarget` _asbp_charisma_player_character)
  (`self.OnMessageResolve`)
  (return))

(fn `InterpretMessageAsSpectator`
  (params (MessageEvent :type "CharismaMessageEvent Structure"))
  (bind _asbp_plug_nplay_game_mode_template (cast `/CharismaPlugNPlay/Blueprint/GameMode/BP_PlugNPlayGameModeTemplate` (`GameplayStatics.GetGameMode`)))
  ;[1 1 1] Look in our entity list for whoever is talking
  (for _array_element (`CharismaPlaythroughInstance.CharismaEntities` (`/CharismaPlugNPlay/Blueprint/GameMode/BP_PlugNPlayGameModeTemplate.CharismaPlaythroughInstance` _asbp_plug_nplay_game_mode_template))
    (if (== (`CharismaEntityComponent.EntityId` _array_element) (`.Name` (break `CharismaCharacter` (`.Character` (break `CharismaMessage` (`.Message` (break `CharismaMessageEvent` MessageEvent)))))))
      ;[1 1 1] Look at that target and resolve the message to progress
      (`self.SetLookAtTarget` (`ActorComponent.GetOwner` _array_element))
      (`self.OnMessageResolve`)
      (return))))

(fn `Register Active Emotion`
  (params (Emotion :type "CharismaEmotion Structure"))
  (for _array_element (`.ActiveEffects` (break `CharismaEmotion` Emotion))
    (bind (_feeling _intensity) (break `CharismaActiveEffect` _array_element))
    (`BlueprintMapLibrary.Map_Add` (`self.EmotionMap`) _feeling _intensity)))

(fn `RequestAnimation`
  (params (animationName :type String))
  (bind (_value _returnvalue) (`BlueprintMapLibrary.Map_Find` (`self.CustomAnims`) animationName))
  (if _returnvalue
    (`AnimInstance.PlaySlotAnimationAsDynamicMontage` (`SkeletalMeshComponent.GetAnimInstance` (`self.Mesh`)) _value "CustomFullbody" 0.25 0.25 1.0 1 -1.0 0.0)))

(fn `SetLookAtTarget`
  (params (Target :type "Actor Object Reference"))
  (if (`KismetSystemLibrary.IsValid` Target)
    (if (not (`KismetSystemLibrary.IsValid` (`self.Look at Target`)))
      (set `self.Look at Target` Target))))

(fn `SetMessageBody`
  (params (Message :type String))
  (set `self.Message` Message))

(fn `SetMoveToTarget`
  (params (MoveToTarget :type "Actor Object Reference"))
  (set `self.MoveToTarget` MoveToTarget))

(fn `SetSpeechData`
  (params (Speech :type "CharismaSpeech Structure"))
  (set `self.Speech` Speech))

(fn `UserConstructionScript`)